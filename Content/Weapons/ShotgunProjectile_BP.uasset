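; Shotgun projectile that applies fixed damage to any actor it begins overlapping and handles surface impacts on hit.
; On hit, it prints the physical material's name and uses it as a Wwise switch for the bullet impact sound.
; It then attaches a short-lived bullet hole decal to the hit component, oriented to the surface normal with random spin, and destroys itself.
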(event `self.ReceiveActorBeginOverlap`
  (params (OtherActor :type "Actor Object Reference"))
  ;[1 1 1] Damage
  (`GameplayStatics.ApplyDamage` OtherActor 25.0))

(event `self.ReceiveHit`
  (params (MyComp :type "PrimitiveComponent Object Reference") (Other :type "Actor Object Reference") (OtherComp :type "PrimitiveComponent Object Reference") (bSelfMoved :type Boolean) (HitLocation :type "Vector Structure") (HitNormal :type "Vector Structure") (NormalImpulse :type "Vector Structure") (Hit :type "HitResult Structure (by ref)"))
  (bind _returnvalue (`KismetMathLibrary.RandomFloatInRange` 0.0 360.0))
  (bind _returnvalue_2 (`KismetStringLibrary.Conv_ObjectToString` (`.PhysMat` (`GameplayStatics.BreakHitResult` Hit))))
  (bind (_x _y _z) (`KismetMathLibrary.BreakRotIntoAxes` (`KismetMathLibrary.Conv_VectorToRotator` HitNormal)))
  ;[1 1 1] Bullet impact sound
  (`KismetSystemLibrary.PrintString` _returnvalue_2)
  (`AkGameplayStatics.SetSwitch` null self "BulletMaterial" (`KismetStringLibrary.Conv_StringToName` _returnvalue_2))
  (`AkGameplayStatics.PostEvent` "/Game/WwiseAudio/Events/Default_Work_Unit/Weapons/Bullet/BulletImpact.BulletImpact" self)
  (`GameplayStatics.SpawnDecalAttached` "/Game/VFX/Texture_Mats/M_BulletHole.M_BulletHole" (5.0 5.0 5.0) OtherComp "None" HitLocation (`KismetMathLibrary.MakeRotationFromAxes` _x (`KismetMathLibrary.RotateAngleAxis` _y _returnvalue _x) (`KismetMathLibrary.RotateAngleAxis` _z _returnvalue _x)) "KeepWorldPosition" 10.0)
  (`self.K2_DestroyActor`))

(fn `UserConstructionScript`)