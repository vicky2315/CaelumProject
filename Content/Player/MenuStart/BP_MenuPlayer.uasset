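; Player pawn for the start menu, which moves the view to a desk terminal and lets the player interact by clicking.
; After a short delay on BeginPlay, it blends the controller's view target to the first DeskTerminal found.
; Left click runs a debug-drawn line trace forward from the camera and, after a delay, sends InteractMessage to hits implementing the Interact interface.
; The UI-only input and cursor setup is unconnected and never runs.
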(event `self.ReceiveBeginPlay`
  (bind _outactors (`GameplayStatics.GetAllActorsOfClass` "/Game/HUD/Terminal/DeskTerminal.DeskTerminal_C"))
  (`KismetSystemLibrary.Delay` 0.5)
  (`PlayerController.SetViewTargetWithBlend` (`PlayerState.GetPlayerController` (`Pawn.PlayerState` (`GameplayStatics.GetPlayerPawn` 0))) (`|GetArrayItem` _outactors) 2.0 "VTBlend_Linear" 0.0 false))

(event `Key|LeftMouseButton`
  (params (Key :type "Key Structure"))
  (bind (_returnvalue_location _returnvalue_rotation) (`KismetMathLibrary.BreakTransform` (`SceneComponent.K2_GetComponentToWorld` (`self.Camera`))))
  (:`Pressed`
    (bind _outhit (`KismetSystemLibrary.LineTraceSingleForObjects` :`Start` _returnvalue_location :`End` (+ _returnvalue_location (* (`KismetMathLibrary.GetForwardVector` _returnvalue_rotation) 1000.0)) :`ObjectTypes` (`|MakeArray` "ObjectTypeQuery1" :!type "EObjectTypeQuery Enum") :`DrawDebugType` "Persistent"))
    (bind (_bblockinghit _binitialoverlap _time _distance _location _impactpoint _normal _impactnormal _physmat _hitactor) (`GameplayStatics.BreakHitResult` _outhit))
    (if (`KismetSystemLibrary.DoesImplementInterface` _hitactor "/Game/Player/MenuStart/Interact.Interact_C")
      (`KismetSystemLibrary.Delay` 2.5)
      (message `/Game/Player/MenuStart/Interact.Interact` _hitactor))))

(fn `UserConstructionScript`)