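; Turret enemy Blueprint that detects the player character through pawn sensing and fires projectiles at it.
; On sighting, it turns toward the player, swaps its sprite for a firing flipbook, waits out a timed delay, then spawns a projectile from an arrow component.
; Tick updates a health bar widget and turns it to face the camera.
; DecreaseHealth adds a health delta and destroys the turret at zero or below.
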(event `self.PawnSensing.OnSeePawn`
  (params (Pawn :type "Pawn Object Reference"))
  (cast `/Game/Player/BP_MyMainCharacter` Pawn)
  (`self.K2_SetActorRotation` (`KismetMathLibrary.FindLookAtRotation` (`self.K2_GetActorLocation`) (`self.K2_GetActorLocation` Pawn)))
  (`SceneComponent.SetVisibility` (`self.PaperSprite`) false false)
  (`SceneComponent.SetVisibility` (`self.PaperFlipbook`) true false)
  (`KismetSystemLibrary.Delay` 1.888889)
  (`PaperFlipbookComponent.SetPlaybackPositionInFrames` (`self.PaperFlipbook`) 33 false)
  (`|SpawnActorFromClass` "/Game/Enemies/Enemy_Sprites/Turret/Firing/Turret_Projectile_BP.Turret_Projectile_BP_C" (`SceneComponent.K2_GetComponentToWorld` (`self.Arrow`)) "Undefined" "MultiplyWithRoot" null null))

(event `self.ReceiveTick`
  (params (DeltaSeconds :type "Float (single-precision)"))
  (bind _healthbar (`self.HealthBar`))
  (bind _asturret_health_bp (cast `/Game/Enemies/Enemy_Sprites/Turret/Firing/Turret_Health_BP` (`WidgetComponent.GetWidget` (`self.HealthBar`))))
  (`ProgressBar.SetPercent` (`/Game/Enemies/Enemy_Sprites/Turret/Firing/Turret_Health_BP.Turret_HealthBar` _asturret_health_bp) (/ (`self.Health`) 100.0))
  (`SceneComponent.K2_SetWorldRotation` _healthbar (`KismetMathLibrary.FindLookAtRotation` (`SceneComponent.K2_GetComponentLocation` _healthbar) (`SceneComponent.K2_GetComponentLocation` (`PlayerCameraManager.TransformComponent` (`GameplayStatics.GetPlayerCameraManager` 0)))) false false))

(event `DecreaseHealth`
  (params (MinusHealth :type "Float (double-precision)"))
  (set `self.Health` (+ (`self.Health`) MinusHealth))
  (if (<= (`self.Health`) 0.0)
    (`self.K2_DestroyActor`)))

(fn `UserConstructionScript`)